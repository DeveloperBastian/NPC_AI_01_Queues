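; BP_QueueActor manages a waiting line that actors join, update and leave by name.
; RegisterInQueue adds or updates the caller in parallel name and position arrays, returning its index, front flag and target location.
; The front actor targets the Arrow component, while each follower targets the last stored position of the one ahead.
; LeaveQueue removes the entry from both arrays, and GetArrowDirection exposes the Arrow's normalized forward vector.
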(fn `GetArrowDirection`
  (returns (NormalizedDirection :type "Vector Structure"))
  (return (`KismetMathLibrary.Normal` (`SceneComponent.GetForwardVector` (`self.Arrow`)))))

(fn `LeaveQueue`
  (params (MyName :type String))
  (locals (Position :type Integer))
  ;[1 1 1] Search for given name and remove from both queues
  (bind _output_get (set `local.Position` (`KismetArrayLibrary.Array_Find` (`self.QueuingActorNames`) MyName)))
  (if (`KismetArrayLibrary.Array_IsValidIndex` (`self.QueuingActorNames`) _output_get)
    (`KismetArrayLibrary.Array_Remove` (`self.QueuingActorNames`) (`local.Position`))
    (`KismetArrayLibrary.Array_Remove` (`self.QueuingActorPositions`) (`local.Position`))))

(fn `RegisterInQueue`
  (params (MyName :type String) (MyLocation :type "Vector Structure"))
  (returns (QueueLocation :type "Vector Structure") (OnFront :type Boolean) (QueuePosition :type Integer))
  (bind _returnvalue (`KismetArrayLibrary.Array_Find` (`self.QueuingActorNames`) MyName))
  (bind _returnvalue_2 (`SceneComponent.K2_GetComponentLocation` (`self.Arrow`)))
  ;[1 1 1] Already registered?
  (if (`KismetArrayLibrary.Array_IsValidIndex` (`self.QueuingActorNames`) _returnvalue)
    ;[1 1 1] Update Location
    (`KismetArrayLibrary.Array_Set` (`self.QueuingActorPositions`) _returnvalue MyLocation)
    (set `self.NumerInQueue` _returnvalue)
    (else
      ;[1 1 1] Newly register
      (bind _returnvalue_3 (`KismetArrayLibrary.Array_Add` (`self.QueuingActorNames`) MyName))
      (`KismetArrayLibrary.Array_Add` (`self.QueuingActorPositions`) MyLocation)
      (set `self.NumerInQueue` _returnvalue_3)))
  ;[1 1 1] Front position?
  (if (== (`self.NumerInQueue`) 0)
    ;[1 1 1] Front position, Location changed to Arrow location
    (`KismetArrayLibrary.Array_Set` (`self.QueuingActorPositions`) 0 _returnvalue_2)
    (return _returnvalue_2 true 0)
    (else
      ;[1 1 1] Get position of actor in front of me in queue. Not in Front. Position in queue returned
      (bind _output_get (set `self.PositionToQueue` (`|GetArrayItem` (`self.QueuingActorPositions`) (- (`self.NumerInQueue`) 1))))
      (return _output_get false (`self.NumerInQueue`)))))

(fn `UserConstructionScript`)