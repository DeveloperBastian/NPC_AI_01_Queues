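; NPC character for a queue-and-carry scenario that picks up a colored burden cube and drops it.
; On BeginPlay it starts at fast-walk speed and picks a random burden color, applied as the mesh overlay material.
; ShoulderBurden shows an attached cube in that color; ReleaseBurden hides it, spawns a matching BP_ChamferCube at the NPC and pushes it backward with an impulse.
; A helper switches max walk speed between fast and slow.
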(event `self.ReceiveBeginPlay`
  ;[1 1 1] Start with fast walk
  (`self.Is Fast Walking` true)
  ;[1 1 1] Random Material
  (bind _output_get (set `self.BurdenColor` (`KismetArrayLibrary.Array_Random` (`self.BurdenColors`))))
  (`MeshComponent.SetOverlayMaterial` (`self.Mesh`) _output_get))

(fn `Is Fast Walking`
  (params (FastWalking :type Boolean))
  (bind _charactermovement (`self.CharacterMovement`))
  (if FastWalking
    (set `CharacterMovementComponent.MaxWalkSpeed` 400.0 _charactermovement)
    (else
      (set `CharacterMovementComponent.MaxWalkSpeed` 150.0 _charactermovement))))

(fn `ReleaseBurden`
  ;[1 1 1] Make rucksack visible
  (`SceneComponent.SetVisibility` (`self.SM_ChamferCube`) false false)
  ;[1 1 1] Spawn cube
  (bind _returnvalue (`|SpawnActorFromClass` "/Game/QueueAndCarry/Blueprints/BP_ChamferCube.BP_ChamferCube_C" (`self.GetTransform` self) "Undefined" "MultiplyWithRoot" null null))
  (`|ExecutionSequence`
    (:`then_0`
      (bind _sm_cube (`/Game/QueueAndCarry/Blueprints/BP_ChamferCube.SM_Cube` _returnvalue))
      ;[1 1 1] Change Color
      (`PrimitiveComponent.SetMaterial` _sm_cube 0 (`self.BurdenColor`)))
    (:`then_1`
      ;[1 1 1] Push away
      (`PrimitiveComponent.AddVelocityChangeImpulseAtLocation` _sm_cube (* (`self.GetActorForwardVector` self) -5.0) (`self.K2_GetActorLocation` self) "None"))))

(fn `ShoulderBurden`
  ;[1 1 1] Random Material
  (`PrimitiveComponent.SetMaterial` (`self.SM_ChamferCube`) 0 (`self.BurdenColor`))
  ;[1 1 1] Make burden visibke
  (`SceneComponent.SetVisibility` (`self.SM_ChamferCube`) true false))

(fn `UserConstructionScript`)