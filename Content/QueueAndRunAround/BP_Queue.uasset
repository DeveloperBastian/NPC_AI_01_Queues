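; Queue actor that lines customers up along a spline, giving each one a place to stand.
; Queue adds the customer uniquely to an array, or finds its existing index, then returns the world location and rotation at index times the given spacing along the spline.
; DeQueue removes a customer, so those behind get closer positions when they next call Queue.
; BeginPlay runs a "show splines" console command for visualization.
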(event `self.ReceiveBeginPlay`
  (`KismetSystemLibrary.ExecuteConsoleCommand` "show splines" null))

(fn `DeQueue`
  (params (CustomerName :type String))
  (`KismetArrayLibrary.Array_RemoveItem` (`self.CustomerQueue`) CustomerName))

(fn `Queue`
  (params (CustomerName :type String) (Distance :type Integer))
  (returns (Location :type "Vector Structure") (Rotation :type "Rotator Structure"))
  (locals (Position :type Integer) (TotalDistance :type "Float (double-precision)"))
  (bind _spline (`self.Spline`))
  (`|ExecutionSequence`
    (:`then_0`
      ;[1 1 1] Add to queue, set position. If already there (INDEX_NONE = -1), then find and set position
      (bind _returnvalue (`KismetArrayLibrary.Array_AddUnique` (`self.CustomerQueue`) CustomerName))
      (bind _output_get (set `local.Position` _returnvalue))
      (if (== _output_get -1)
        (set `local.Position` (`KismetArrayLibrary.Array_Find` (`self.CustomerQueue`) CustomerName))))
    (:`then_1`
      ;[1 1 1] Calculate total distance, return location and rotation at this point in spline
      (bind _output_get_2 (set `local.TotalDistance` (`KismetMathLibrary.Conv_IntToDouble` (* Distance (`local.Position`)))))
      (return (`SplineComponent.GetLocationAtDistanceAlongSpline` _spline _output_get_2 "World") (`SplineComponent.GetRotationAtDistanceAlongSpline` _spline _output_get_2 "World")))))

(fn `UserConstructionScript`)